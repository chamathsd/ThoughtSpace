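; ThoughtSpaceProxy is a Blueprint that tests Leap Motion grab input with a camera-based object trace.
; Pressing either hand's grab prints a message, then line-traces forward from the player camera manager for WorldDynamic objects, with debug drawing.
; It only prints whether the trace hit; nothing is picked up or moved.
; Releasing either grab just prints a message.
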(event `self.ReceiveBeginPlay`
  (`parent.ReceiveBeginPlay`))

(event `self.ReceiveActorBeginOverlap`
  (params (OtherActor :type "Actor Object Reference")))

(event `Key|LeapLeftGrab`
  (bind _returnvalue (`GameplayStatics.GetPlayerCameraManager` 0))
  (bind _returnvalue_2 (`self.K2_GetActorLocation` _returnvalue))
  (:`Pressed`
    (`KismetSystemLibrary.PrintString` "Grabbed" :!label _label)
    (bind (_outhit _returnvalue_3) (`KismetSystemLibrary.LineTraceSingleForObjects` :`Start` _returnvalue_2 :`End` (+ _returnvalue_2 (* (`KismetMathLibrary.GetForwardVector` (`self.K2_GetActorRotation` _returnvalue)) 1500.0)) :`ObjectTypes` (`|MakeArray` "ObjectTypeQuery2" :!type "EngineTypes.EObjectTypeQuery Enum") :`DrawDebugType` "ForOneFrame"))
    (`KismetSystemLibrary.PrintString` (`KismetStringLibrary.Conv_BoolToString` _returnvalue_3)))
  (:`Released`
    (`KismetSystemLibrary.PrintString` "Released" true false :!label _label_2)))

(event `Key|LeapRightGrab`
  (:`Pressed`
    (goto _label))
  (:`Released`
    (goto _label_2)))

(fn `UserConstructionScript`
  (`parent.UserConstructionScript`))